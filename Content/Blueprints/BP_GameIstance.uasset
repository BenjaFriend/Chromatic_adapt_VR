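; Game instance Blueprint that reports players' "Grey" picks per level to a remote server and cycles through levels.
; It loads the Scrutiny reporting DLL from a plugin folder, initialises it with a server address, and releases and frees it on end play.
; SelectedGrey sends each selection with the current level name as a key-value report.
; NextLevel advances through the LevelIndex array, wrapping to the first entry after the last.
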(event `CustomEvent_1`
  ;[1 1 1] Import Scrutiny (a DLL in plugins folder)
  (bind _returnvalue (`ScrutinyBFL.importDLL` "Scrutiny" "Scrutiny.dll"))
  (if _returnvalue
    ;[1 1 1] Import and init the lib
    (bind _returnvalue_2 (`ScrutinyBFL.ImportScrutiny`))
    (if _returnvalue_2
      (`KismetSystemLibrary.PrintString` "Imported Scrutiny!")
      (`ScrutinyBFL.getInitLibFromDll` "benjafriend.hopto.org" "9222")
      (else
        (`KismetSystemLibrary.PrintString` "Importing method Init Lib failed!")))
    (else
      (`KismetSystemLibrary.PrintString` "Importing DLL failed!"))))

(event `CustomEvent`
  (params (EndPlayReason :type "EEndPlayReason Enum" :default "Destroyed"))
  ;[1 1 1] release Scrutiny (clean up DLL)
  (`|ExecutionSequence`
    (:`then_0`
      (`ScrutinyBFL.getReleaseFromDll`))
    (:`then_1`
      (`ScrutinyBFL.freeDLL`))))

(event `SelectedGrey`
  (params (Selection :type String))
  ;[1 1 1] Event to handle reporting of which Grey the user though was correct for a level
  (`KismetSystemLibrary.PrintString` Selection)
  (`ScrutinyBFL.getStartReportFromDll`)
  ;;[1 1 1] Report which grey is selected
  (`ScrutinyBFL.getReportCharacterFromDll` "GreySelection" Selection)
  ;;[1 1 1] report level name
  (bind _returnvalue (`GameplayStatics.GetCurrentLevelName` true))
  (`ScrutinyBFL.getReportCharacterFromDll` "LevelName" _returnvalue)
  (`ScrutinyBFL.getSendReportFromDll`))

(fn `NextLevel`
  ;[1 1 1] Increment level index, clamping to max array size
  (bind _result (`/Engine/EditorBlueprintResources/StandardMacros.IncrementInt` (`self.CurrentLevelIndex`))
    (:`  `
      (if (> _result (- (`KismetArrayLibrary.Array_Length` (`self.LevelIndex`)) 1))
        (set `self.CurrentLevelIndex` 0)
        (else
          (set `self.CurrentLevelIndex` _result)))
      (`KismetSystemLibrary.PrintString` "Load Level Index ^^")
      ;[1 1 1] Open Level at index
      (`GameplayStatics.OpenLevel` (`|GetArrayItem` (`self.LevelIndex`) (`self.CurrentLevelIndex`))))))